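; Bonus card actor for combat that grants bonus card draws when the player consumes a required set of items within a turn.
; On BeginPlay it maps the card's item requirements and adds a WBP_BonusCard widget to the combat UI.
; Tick rebuilds the turn's consumed-item map from the player character and updates clamped progress.
; Meeting all requirements draws the bonus through the item deck once, re-armed at player turn start.
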(event EventBeginPlay
  (Utilities|FlowControl|Delay 0.1)
  (Variables|Default|Setstart true)
  (bind _itemmap1 (CallFunction|ItemNumArraytoMap (.ItemNeed (Utilities|Struct|BreakST_BonusCard (Variables|Default|GetST_BonusCard)))))
  (Variables|Default|SetNeedItemMap _itemmap1)
  (bind _asbp_top_down_character (Utilities|Casting|CastToBP_TopDownCharacter (Game|GetPlayerCharacter 0)))
  (bind _returnvalue (UserInterface|CreateWidget "/Game/SalesGirl/UI/WBP_BonusCard.WBP_BonusCard_C" 0 (Variables|Default|GetST_BonusCard)))
  (Class|VerticalBox|AddChildtoVerticalBox (Variables|/Game/SalesGirl/UI/WBP_CombatMain.WBP_CombatMain_C|GetVerticalBox_BonusCard (Variables|/Game/SalesGirl/Character/BP_TopDownCharacter.BP_TopDownCharacter_C|GetCombatUIRef _asbp_top_down_character)) _returnvalue)
  (Variables|Default|SetBonusCardUi _returnvalue))

(event Collision|EventActorBeginOverlap
  (params (OtherActor :type Actor%20Object%20Reference)))

(event EventTick
  (params (DeltaSeconds :type Float%20%28single-precision%29))
  (if (Variables|Default|Getstart)
    (CallFunction|SetProgress)
    (CallFunction|TickInitial)
    (bind _conditionmeet (CallFunction|IsMeetConditon))
    (if _conditionmeet
      (Utilities|FlowControl|DoOnce false
        (:Completed
          (bind _asbp_top_down_character (Utilities|Casting|CastToBP_TopDownCharacter (Game|GetPlayerCharacter 0)))
          (Default|DrawCardsinCombat (Variables|/Game/SalesGirl/Character/BP_TopDownCharacter.BP_TopDownCharacter_C|GetItemDeckRef _asbp_top_down_character) (.CardBonus (Utilities|Struct|BreakST_BonusCard (Variables|Default|GetST_BonusCard))))
          (Variables|/Game/SalesGirl/UI/WBP_BonusCard.WBP_BonusCard_C|SetFinished (Variables|Default|GetBonusCardUi) true))))))

(event EventPlayerTurnStartEvent
  (if (Variables|Default|Getstart)
    (Utilities|FlowControl|Sequence
      (:then_0
        (Utilities|FlowControl|DoOnce false) ; enters at Reset
      )
      (:then_1
        (Variables|/Game/SalesGirl/UI/WBP_BonusCard.WBP_BonusCard_C|SetFinished (Variables|Default|GetBonusCardUi) false)))))

(fn ConstructionScript)

(fn IsMeetConditon
  (bind _keys (Utilities|Map|Keys (Variables|Default|GetNeedItemMap)))
  (bind _array_element (Utilities|Array|ForEachLoopwithBreak _keys)
    (:LoopBody
      (if (.ReturnValue (Utilities|Map|Find (Variables|Default|GetTurnConsumedItem%20Map) _array_element))
        (if (not (>= (.Value (Utilities|Map|Find (Variables|Default|GetTurnConsumedItem%20Map) _array_element)) (.Value (Utilities|Map|Find (Variables|Default|GetNeedItemMap) _array_element))))
          (return false))
        (else
          (return false))))
    (:Completed
      (return true))))

(fn TickInitial
  (Utilities|Map|Clear (Variables|Default|GetTurnConsumedItem%20Map))
  (bind _asbp_top_down_character (Utilities|Casting|CastToBP_TopDownCharacter (Game|GetPlayerCharacter 0)))
  (bind _output_get (Variables|Default|SetTurn%20Consumed%20Item (Variables|/Game/SalesGirl/Character/BP_TopDownCharacter.BP_TopDownCharacter_C|GetTurnConsumedItem _asbp_top_down_character)))
  (bind _itemmap1 (CallFunction|ItemSTArraytoMap _output_get))
  (Variables|Default|SetTurnConsumedItem%20Map _itemmap1))

(fn SetProgress
  (bind _values (Utilities|Map|Values (Variables|Default|GetNeedItemMap)))
  (bind _sum1 (CallFunction|IntArraySum _values))
  (bind _keys (Utilities|Map|Keys (Variables|Default|GetNeedItemMap)))
  (bind _array_element (Utilities|Array|ForEachLoopwithBreak _keys)
    (:LoopBody
      (if (.ReturnValue (Utilities|Map|Find (Variables|Default|GetTurnConsumedItem%20Map) _array_element))
        (LocalVariables|SetConsumedItemNum (+ (Math|Integer|Clamp(Integer) (.Value (Utilities|Map|Find (Variables|Default|GetTurnConsumedItem%20Map) _array_element)) 0 (.Value (Utilities|Map|Find (Variables|Default|GetNeedItemMap) _array_element))) (LocalVariables|GetConsumedItemNum)))))
    (:Completed
      (Variables|/Game/SalesGirl/UI/WBP_BonusCard.WBP_BonusCard_C|SetProgress (Variables|Default|GetBonusCardUi) (Math|Float|SafeDivide (Math|Conversions|ToFloat(Integer) (LocalVariables|GetConsumedItemNum)) (Math|Conversions|ToFloat(Integer) _sum1)))
      (return))))