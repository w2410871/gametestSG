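; BP_DamagedCharacter is a damageable character that resolves incoming elemental attacks and displays pop-up damage text.
; On BeginPlay it caches the main canvas from its damage widget component's UI panel.
; SGApplydamage runs a shared hit, evasion and resistance calculation, subtracting received damage from current HP on a hit.
; Hits and misses spawn pop-up widgets on that canvas, with hit pop-ups tiered by the sign of the element's resistance.
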(event EventBeginPlay
  (bind _aswbp_damage_character_uipanel (Utilities|Casting|CastToWBP_DamageCharacterUIPanel (UserInterface|GetWidget (Variables|Default|GetDamageCharacterWidget)))
    (:then
      (Variables|Default|SetMain%20Canvas (Variables|/Game/SalesGirl/UI/WBP_DamageCharacterUIPanel.WBP_DamageCharacterUIPanel_C|GetMainCanvas _aswbp_damage_character_uipanel))
      (Development|PrintString "set"))
    (:CastFailed
      (Development|PrintString "cast fail"))))

(event EventSGApplydamage
  (params (Damage :type Float%20%28double-precision%29) (Hitrate :type Float%20%28double-precision%29) (ElementTyoe :type ElementType%20Enum :default "NewEnumerator2"))
  (bind _elementresist (Variables|Default|GetElementResist))
  (bind _value (Utilities|Map|Find _elementresist ElementTyoe))
  (bind (_ishit _receivedamage) (CallFunction|DamageCal Hitrate (Variables|Default|GetEvasionRate) Damage _value self))
  (if _ishit
    (Variables|Default|SetCurrentHP (- (Variables|Default|GetCurrentHP) _receivedamage))
    (bind _elementrisitlevel (CallFunction|GetRisistlevel _value))
    (bind _returnvalue (UserInterface|CreateWidget "/Game/SalesGirl/UI/DamagePopUp.DamagePopUp_C" 0 false _elementrisitlevel _receivedamage))
    (Widget|Panel|AddChild (Variables|Default|GetMain%20Canvas) _returnvalue)
    (Default|PopUpText _returnvalue)
    (else
      (Development|PrintString "miss")
      (bind _returnvalue_2 (UserInterface|CreateWidget "/Game/SalesGirl/UI/DamagePopUp.DamagePopUp_C" 0 true "NewEnumerator1"))
      (Widget|Panel|AddChild (Variables|Default|GetMain%20Canvas) _returnvalue_2)
      (Default|PopUpText _returnvalue_2))))

(fn ConstructionScript)

(fn GetRisistlevel
  (params (ElementRisit :type Float%20%28double-precision%29))
  (if (> ElementRisit 0.0)
    (return "NewEnumerator2")
    (elif (== ElementRisit 0.0)
      (return "NewEnumerator1")
      (else
        (return "NewEnumerator0")))))