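; BP_Monster is an enemy in turn-based combat that fires projectiles at the player on its turn.
; On BeginPlay it loads its stats from DT_Monster by MonsterID, links its HP bar widget to itself and caches the ProcessController.
; ActionStart spawns a bullet aimed at the player, carrying damage, element and a distance-based hit rate, then notifies the controller after a short delay.
; PlayerTurnStartEvent clears its acted flag.
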(event Custom|Fire
  (bind _returnvalue (Game|GetPlayerCharacter 0))
  (Game|SpawnActorfromClass (Variables|Default|GetBullet%20Class) (Math|Transform|MakeTransform (+ (* (Transformation|GetActorForwardVector) (Math|Float|MakeLiteralFloat 5e+01)) (Transformation|GetActorLocation)) (Math|Rotator|FindLookatRotation (Transformation|GetActorLocation) (Transformation|GetActorLocation _returnvalue)) "1.000000,1.000000,1.000000") "Undefined" "MultiplyWithRoot" 0 (Math|Float|Truncate (Variables|Default|GetDamage)) _returnvalue (.Value (Utilities|Map|Find (Variables|Default|GetHITRate%20Dis) (Variables|/Game/SalesGirl/ProcessController.ProcessController_C|GetDistance (Variables|Default|GetProcessCtrRef)))) (Variables|Default|GetAttack%20Element) 0))

(event Custom|ActionStart
  (CallFunction|Fire)
  (Variables|Default|SetActed true)
  (Utilities|FlowControl|Delay 0.5)
  (Default|SingleMonsterEnd1 (Variables|Default|GetProcessCtrRef)))

(event EventBeginPlay
  (|CallParentFunction)
  (bind _returnvalue (Utilities|GetDataTableRow "/Game/SalesGirl/Datatable/DT_Monster.DT_Monster" (Utilities|String|StringToName (Variables|Default|GetMonsterID)))
    (:then
      (Variables|Default|SetDamage (.Damage (Utilities|Struct|BreakST_Monster _returnvalue)))
      (bind _output_get (Variables|Default|SetMAXHP (.HP (Utilities|Struct|BreakST_Monster _returnvalue))))
      (Variables|Default|SetCurrentHP _output_get)
      (Variables|Default|SetElementResist (.ElementResistance (Utilities|Struct|BreakST_Monster _returnvalue)))
      (Variables|Default|SetHITRate%20Dis (.HITRateDis (Utilities|Struct|BreakST_Monster _returnvalue)))
      (Variables|Default|SetAttack%20Element (.AttackElement (Utilities|Struct|BreakST_Monster _returnvalue)))
      (bind _aswbp_hpbar (Utilities|Casting|CastToWBP_HPBar (UserInterface|GetWidget (Variables|Default|GetWidget_0)))
        (:then
          (Variables|/Game/SalesGirl/UI/WBP_HPBar.WBP_HPBar_C|SetMonsterRef _aswbp_hpbar self)
          (bind _outactors (Actor|GetAllActorsOfClass "/Game/SalesGirl/ProcessController.ProcessController_C"))
          (Variables|Default|SetProcessCtrRef (Utilities|Array|Get(acopy) _outactors)))
        (:CastFailed
          (Development|PrintString "cast fail"))))
    (:RowNotFound
      (Development|PrintString "没有找到怪物配置"))))

(event EventPlayerTurnStartEvent
  (Variables|Default|SetActed false))

(fn ConstructionScript)