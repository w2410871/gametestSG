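; Base weapon actor that charges up from items and fires a projectile once its item cost is met.
; BeginPlay loads cost, bullet class and damage from DT_WeaponData by WeaponID, adds a widget to the player's combat UI, then starts disabled.
; While enabled, BasicFire decrements the matching item count and highlights its icon.
; When all counts reach zero, Fire spawns the bullet toward the nearest BP_Monster, or actor-forward without one, and refills the cost.
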(event Custom|Fire
  (bind _output (CallFunction|MinDistanceActortoSource "/Game/TopDown/Blueprints/BP_Monster.BP_Monster_C" self))
  (Utilities|IsValid _output
    (:Is%20Valid
      (Variables|Default|SetSpawn%20Transform%20Rotation (Math|Rotator|FindLookatRotation (Transformation|GetActorLocation) (Transformation|GetActorLocation _output))))
    (:Is%20Not%20Valid
      (Variables|Default|SetSpawn%20Transform%20Rotation (Transformation|GetActorRotation))))
  (Game|SpawnActorfromClass (Variables|Default|GetBullet%20Class) (Math|Transform|MakeTransform (+ (* (Transformation|GetActorForwardVector) (Math|Float|MakeLiteralFloat 5e+01)) (Transformation|GetActorLocation)) (Variables|Default|GetSpawn%20Transform%20Rotation) "1.000000,1.000000,1.000000") "Undefined" "MultiplyWithRoot" 0 (Variables|Default|GetWeapon%20Damage) _output 0)
  (Variables|Default|SetItemRemain (Variables|Default|GetItemCostMap))
  (Default|Reset (Variables|Default|GetWeaponUIRef)))

(event Custom|reset
  (CallFunction|SetWeaponEnable false)
  (Variables|Default|SetItemRemain (Variables|Default|GetItemCostMap))
  (Default|Reset (Variables|Default|GetWeaponUIRef)))

(event EventBeginPlay
  (Utilities|FlowControl|DelayUntilNextTick)
  (bind _returnvalue (Utilities|GetDataTableRow "/Game/SalesGirl/Datatable/DT_WeaponData.DT_WeaponData" (Utilities|String|StringToName (Variables|Default|GetWeaponID)))
    (:then
      (bind _output_get (Variables|Default|SetItem%20Cost (.ItemCost (Utilities|Struct|BreakSt_Weapon _returnvalue))))
      (Variables|Default|SetBullet%20Class (.BulletClass (Utilities|Struct|BreakSt_Weapon _returnvalue)))
      (Variables|Default|SetWeapon%20Damage (.WeaponDamage (Utilities|Struct|BreakSt_Weapon _returnvalue)))
      (bind _itemmap1 (CallFunction|ItemNumArraytoMap _output_get))
      (bind _output_get_2 (Variables|Default|SetItemCostMap _itemmap1))
      (Variables|Default|SetItemRemain _output_get_2)
      (bind _returnvalue_2 (UserInterface|CreateWidget "/Game/SalesGirl/UI/WBP_weapon.WBP_weapon_C" 0 (Variables|Default|GetWeaponID)))
      (Variables|Default|SetWeaponUIRef _returnvalue_2)
      (bind _asbp_top_down_character (Utilities|Casting|CastToBP_TopDownCharacter (Game|GetPlayerCharacter 0)))
      (Class|HorizontalBox|AddChildtoHorizontalBox (Variables|/Game/SalesGirl/UI/WBP_CombatMain.WBP_CombatMain_C|GetHorizontalBox_Weapon (Variables|/Game/TopDown/Blueprints/BP_TopDownCharacter.BP_TopDownCharacter_C|GetCombatUIRef _asbp_top_down_character)) _returnvalue_2)
      (CallFunction|SetWeaponEnable false))
    (:RowNotFound
      (Development|PrintString "BP_WEAPON 未找到配置"))))

(event Collision|EventActorBeginOverlap
  (params (OtherActor :type Actor%20Object%20Reference)))

(event EventTick
  (params (DeltaSeconds :type Float%20%28single-precision%29)))

(event EventBasicFire
  (params (ST_item :type St%20Item%20Structure))
  (bind _itemid (Utilities|Struct|BreakSt_Item ST_item))
  (bind _itemremain (Variables|Default|GetItemRemain))
  (bind (_value _returnvalue) (Utilities|Map|Find _itemremain _itemid))
  (if (Variables|Default|GetEnable)
    (if _returnvalue
      (if (!= _value 0)
        (Utilities|Map|Add _itemremain _itemid (- _value 1))
        (Default|HighlightIcon (Variables|Default|GetWeaponUIRef) _itemid)
        (bind _values (Utilities|Map|Values (Variables|Default|GetItemRemain)))
        (bind _true (CallFunction|IsAllElementtoInt _values))
        (if _true
          (CallFunction|Fire))))))

(fn ConstructionScript)

(fn SetWeaponEnable
  (params (Enable :type Boolean))
  (if Enable
    (Rendering|SetVisibility (Variables|Default|GetCube) true false)
    (Widget|SetVisibility (Variables|Default|GetWeaponUIRef) "SelfHitTestInvisible")
    (Variables|Default|SetEnable true)
    (else
      (Rendering|SetVisibility (Variables|Default|GetCube) false false)
      (Widget|SetVisibility (Variables|Default|GetWeaponUIRef) "Collapsed")
      (Variables|Default|SetEnable false))))